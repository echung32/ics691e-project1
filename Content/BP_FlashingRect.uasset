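; BP_FlashingRect is an actor that makes its static mesh blink on and off in game.
; BeginPlay starts a timer that calls CycleHiddenState after a short delay.
; CycleHiddenState toggles the mesh's hidden state using CurrentIndex, then re-arms its own timer, keeping the mesh visible longer than it stays hidden when shown.
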(event Custom|CycleHiddenState
  (bind _staticmeshcomponent (Variables|Debug|GetStaticMeshComponent))
  (if (== (Variables|Default|GetCurrentIndex) 0)
    (Development|SetHiddeninGame _staticmeshcomponent false false)
    (Variables|Default|SetCurrentIndex 1)
    (Utilities|Time|SetTimerbyEvent (delegate Custom|CycleHiddenState) 3.0)
    (else
      (Development|SetHiddeninGame _staticmeshcomponent true false)
      (Variables|Default|SetCurrentIndex 0)
      (Utilities|Time|SetTimerbyEvent (delegate Custom|CycleHiddenState) 2.0))))

(event Collision|EventActorBeginOverlap
  (params (OtherActor :type Actor%20Object%20Reference)))

(event EventTick
  (params (DeltaSeconds :type Float%20%28single-precision%29)))

(event EventBeginPlay
  (Utilities|Time|SetTimerbyEvent (delegate Custom|CycleHiddenState) 2.0))

(fn ConstructionScript)